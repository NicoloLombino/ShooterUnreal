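; BP_DeadZonePlayer is a dead-zone volume that affects the health of a BP_PlayerBaseDoozy player standing inside it.
; Cube overlap events cast to that class, storing the player and setting HasPlayer on entry, then clearing the flag on exit.
; While the flag is set, Tick runs a half-second Delay before calling SetHealth on the player with a fixed value, so the call repeats periodically.
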(event OnComponentBeginOverlap(Cube)
  (params (OverlappedComponent :type Primitive%20Component%20Object%20Reference) (OtherActor :type Actor%20Object%20Reference) (OtherComp :type Primitive%20Component%20Object%20Reference) (OtherBodyIndex :type Integer) (bFromSweep :type Boolean) (SweepResult :type Hit%20Result%20Structure%20%28by%20ref%29))
  (bind _asbp_player_base_doozy (Utilities|Casting|CastToBP_PlayerBaseDoozy OtherActor))
  (Variables|Default|SetPlayer _asbp_player_base_doozy)
  (Variables|Default|SetHasPlayer true))

(event OnComponentEndOverlap(Cube)
  (params (OverlappedComponent :type Primitive%20Component%20Object%20Reference) (OtherActor :type Actor%20Object%20Reference) (OtherComp :type Primitive%20Component%20Object%20Reference) (OtherBodyIndex :type Integer))
  (Utilities|Casting|CastToBP_PlayerBaseDoozy OtherActor)
  (Variables|Default|SetHasPlayer false))

(event EventTick
  (params (DeltaSeconds :type Float%20%28single-precision%29))
  (if (and (Variables|Default|GetHasPlayer) (Utilities|IsValid (Variables|Default|GetPlayer)))
    (Utilities|FlowControl|Delay 0.5)
    (Class|PlayerBase|SetHealth (Variables|Default|GetPlayer) 1.0)))

(fn ConstructionScript)