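; BP_TurnLightOn is an interactable actor with a box trigger and two spotlights, apparently a light switch given its name.
; BeginPlay stores the box in BoxCollision and both spotlights in the Lights array.
; Box overlaps set a BP_PlayerBaseDoozy player's InteractionActor to this actor on entry and clear it on exit.
; The graph itself contains no logic that switches the lights.
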(event OnComponentBeginOverlap(Box)
  (params (OverlappedComponent :type Primitive%20Component%20Object%20Reference) (OtherActor :type Actor%20Object%20Reference) (OtherComp :type Primitive%20Component%20Object%20Reference) (OtherBodyIndex :type Integer) (bFromSweep :type Boolean) (SweepResult :type Hit%20Result%20Structure%20%28by%20ref%29))
  (bind _asbp_player_base_doozy (Utilities|Casting|CastToBP_PlayerBaseDoozy OtherActor))
  (Variables|/Game/CoseMie/Actors/Doozy/BP_PlayerBaseDoozy.BP_PlayerBaseDoozy_C|SetInteractionActor _asbp_player_base_doozy self))

(event OnComponentEndOverlap(Box)
  (params (OverlappedComponent :type Primitive%20Component%20Object%20Reference) (OtherActor :type Actor%20Object%20Reference) (OtherComp :type Primitive%20Component%20Object%20Reference) (OtherBodyIndex :type Integer))
  (bind _asbp_player_base_doozy (Utilities|Casting|CastToBP_PlayerBaseDoozy OtherActor))
  (Variables|/Game/CoseMie/Actors/Doozy/BP_PlayerBaseDoozy.BP_PlayerBaseDoozy_C|SetInteractionActor _asbp_player_base_doozy 0))

(event EventBeginPlay
  (Variables|Default|SetBoxCollision (Variables|Default|GetBox))
  (Variables|Default|SetLights (Utilities|Array|MakeArray (Variables|Default|GetSpotLight) (Variables|Default|GetSpotLight1))))

(fn ConstructionScript)