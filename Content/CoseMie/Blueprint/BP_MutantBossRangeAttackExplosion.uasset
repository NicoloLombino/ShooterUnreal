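; Delayed explosion for the mutant boss's ranged attack that affects the player's health.
; A timeline grows the sphere from zero to its initial scale, then swaps it for a slowed explosion particle with sound and enables collision overlap events.
; An overlapping player gets a SetHealth call and the collision is destroyed, limiting it to one hit.
; A timer started at BeginPlay also removes the collision, closing the hit window.
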(event OnComponentBeginOverlap(SphereCollision)
  (params (OverlappedComponent :type Primitive%20Component%20Object%20Reference) (OtherActor :type Actor%20Object%20Reference) (OtherComp :type Primitive%20Component%20Object%20Reference) (OtherBodyIndex :type Integer) (bFromSweep :type Boolean) (SweepResult :type Hit%20Result%20Structure%20%28by%20ref%29))
  (bind _asbp_player_base_doozy (Utilities|Casting|CastToBP_PlayerBaseDoozy OtherActor))
  (Class|PlayerBase|SetHealth _asbp_player_base_doozy 2e+01)
  (Components|DestroyComponent (Variables|Default|GetSphereCollision)))

(event Custom|DestroyThis
  (Components|DestroyComponent (Variables|Default|GetSphereCollision)))

(event EventBeginPlay
  (Utilities|Time|SetTimerbyEvent (delegate Custom|DestroyThis) 1.5)
  (Variables|Default|SetStartScale (Transformation|GetWorldScale (Variables|Default|GetSphere)))
  (bind _newtrack_0 (Timeline|Timeline_0 PlayFromStart)
    (:Update
      (Transformation|SetRelativeScale3D (Variables|Default|GetSphere) (Math|Vector|Lerp(Vector) "0, 0, 0" (Variables|Default|GetStartScale) _newtrack_0)))
    (:Finished
      (Components|DestroyComponent (Variables|Default|GetSphere))
      (bind _returnvalue (Effects|SpawnEmitteratLocation "/Game/ContenutiIniziali/Particles/P_Explosion.P_Explosion" (Transformation|GetWorldLocation (Variables|Default|GetDefaultSceneRoot)) "0, 0, 0" "4.000000,4.000000,4.000000"))
      (Audio|PlaySound2D "/Game/ContenutiIniziali/Audio/Explosion02.Explosion02" 1.0 1.0 0.0 0 0)
      (Variables|/Script/Engine.ParticleSystemComponent|SetCustomTimeDilation _returnvalue 0.5)
      (Variables|/Script/Engine.PrimitiveComponent|SetbGenerateOverlapEvents (Variables|Default|GetSphereCollision) true))))

(fn ConstructionScript)