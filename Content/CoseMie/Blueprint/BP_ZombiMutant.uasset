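; Zombie mutant enemy Blueprint with a melee attack, a vomit area attack and a health bar widget it can show or hide.
; While alive and in range, Tick faces the target and randomly plays the melee or rarer vomit montage section, gated by a cooldown.
; A toggleable sphere reports melee hits.
; A timeline grows and advances the vomit particles and second sphere, which notifies players entering or leaving to handle damage over time.
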(event OnComponentBeginOverlap(Sphere)
  (params (OverlappedComponent :type Primitive%20Component%20Object%20Reference) (OtherActor :type Actor%20Object%20Reference) (OtherComp :type Primitive%20Component%20Object%20Reference) (OtherBodyIndex :type Integer) (bFromSweep :type Boolean) (SweepResult :type Hit%20Result%20Structure%20%28by%20ref%29))
  (Class|EnemyMonster|AttackCollisionHit OtherActor (Variables|Default|Getdamage)))

(event OnComponentBeginOverlap(Sphere1)
  (params (OverlappedComponent :type Primitive%20Component%20Object%20Reference) (OtherActor :type Actor%20Object%20Reference) (OtherComp :type Primitive%20Component%20Object%20Reference) (OtherBodyIndex :type Integer) (bFromSweep :type Boolean) (SweepResult :type Hit%20Result%20Structure%20%28by%20ref%29))
  (bind _asbp_player_base_doozy (Utilities|Casting|CastToBP_PlayerBaseDoozy OtherActor))
  (Class|PlayerBase|HandleEnteronVomitArea _asbp_player_base_doozy (Variables|Default|GetVomitDamage) (Variables|Default|GetVomitDamageRateTime)))

(event OnComponentEndOverlap(Sphere1)
  (params (OverlappedComponent :type Primitive%20Component%20Object%20Reference) (OtherActor :type Actor%20Object%20Reference) (OtherComp :type Primitive%20Component%20Object%20Reference) (OtherBodyIndex :type Integer))
  (bind _asbp_player_base_doozy (Utilities|Casting|CastToBP_PlayerBaseDoozy OtherActor))
  (Class|PlayerBase|HandleExitfromVomitArea _asbp_player_base_doozy))

(event Custom|SetAttackCollider
  (params (Generate%20Overlap%20Events :type Boolean))
  (Variables|/Script/Engine.PrimitiveComponent|SetbGenerateOverlapEvents (Variables|Default|GetSphere) Generate%20Overlap%20Events))

(event Custom|LookAtTarget
  (bind _target (Variables|Default|GetTarget))
  (bind _capsulecomponent (Variables|Default|GetCapsuleComponent))
  (if (Utilities|IsValid _target)
    (Transformation|SetWorldRotation _capsulecomponent (Math|Rotator|FindLookatRotation (Transformation|GetWorldLocation _capsulecomponent) (Transformation|GetActorLocation _target)) false false)))

(event Custom|HandleVomitAttack
  (bind _sphere1 (Variables|Default|GetSphere1))
  (Rendering|SetVisibility (Variables|Default|GetParticleSystem) true false)
  (Variables|/Script/Engine.PrimitiveComponent|SetbGenerateOverlapEvents (Variables|Default|GetSphere1) true)
  (bind _vomitsize (Timeline|Timeline_0 PlayFromStart)
    (:Update
      (Transformation|SetWorldScale3D (Variables|Default|GetParticleSystem) (Math|Vector|Lerp(Vector) "0, 0, 0" "6.000000,6.000000,6.000000" _vomitsize))
      (Transformation|SetWorldScale3D _sphere1 (Math|Vector|Lerp(Vector) "0, 0, 0" "6.000000,6.000000,6.000000" _vomitsize))
      (Transformation|SetRelativeLocation _sphere1 (Math|Vector|MakeVector 0.0 (Math|Float|Lerp 4e+01 3.3e+02 _vomitsize) 1.5e+02) false false))
    (:Finished
      (CallFunction|ResetVomit))))

(event Custom|StopVomitAttack
  (Rendering|SetVisibility (Variables|Default|GetParticleSystem) false false)
  (Variables|/Script/Engine.PrimitiveComponent|SetbGenerateOverlapEvents (Variables|Default|GetSphere1) false))

(event Custom|ResetVomit
  (bind _sphere1 (Variables|Default|GetSphere1))
  (Transformation|SetWorldScale3D (Variables|Default|GetParticleSystem) "1.000000,1.000000,1.000000")
  (Transformation|SetWorldScale3D _sphere1 "1.000000,1.000000,1.000000")
  (Transformation|SetRelativeLocation _sphere1 "0,70.000000,150.000000" false false))

(event EventBeginPlay
  (bind _asbp_enemy_widget_life (Utilities|Casting|CastToBP_EnemyWidgetLife (UserInterface|GetUserWidgetObject (Variables|Default|GetHealthBar))))
  (Variables|/Game/CoseMie/UI/BP_EnemyWidgetLife.BP_EnemyWidgetLife_C|SetEnemy _asbp_enemy_widget_life self)
  (Widget|SetVisibility (UserInterface|GetUserWidgetObject (Variables|Default|GetHealthBar)) "Hidden"))

(event Collision|EventActorBeginOverlap
  (params (OtherActor :type Actor%20Object%20Reference)))

(event EventTick
  (params (DeltaSeconds :type Float%20%28single-precision%29))
  (if (> (Variables|Default|GetcurrentHealth) 0.0)
    (if (Variables|Default|GetisInAttackRange)
      (if (Variables|Default|GetCanAttack)
        (Variables|Default|SetCanAttack false)
        (CallFunction|LookatTarget)
        (switch int (Math|Random|RandomIntegerinRange 0 2)
          (:Default
            (Animation|PlayAnimMontage "/Game/CoseMie/Actors/ZombiLikeMixamo/AM_ZombiMutantAttack1.AM_ZombiMutantAttack1" 1.0 "Vomit" :!label _label)
            (Audio|PlaySound2D "/Game/CoseMie/Actors/AlienMixamo/Sound/alien_roar_2.alien_roar_2" 1.0 1.0 0.0 0 0)
            (Utilities|FlowControl|Delay (+ 5.0 (Variables|Default|GetVomitAttackTimer)))
            (Variables|Default|SetCanAttack true))
          (:0
            (Animation|PlayAnimMontage "/Game/CoseMie/Actors/ZombiLikeMixamo/AM_ZombiMutantAttack1.AM_ZombiMutantAttack1" 1.0 "Attack" :!label _label_2)
            (Audio|PlaySound2D "/Game/CoseMie/Sounds/Enemies/Zombi/614068__stormwaveaudio__demon-pain-1.614068__stormwaveaudio__demon-pain-1" 1.0 1.0 0.0 0 0)
            (Utilities|FlowControl|Delay (+ 3.0 (Variables|Default|GetAttackTimer)))
            (Variables|Default|SetCanAttack true))
          (:1
            (goto _label_2))
          (:2
            (goto _label)))))))

(event EventShowHealthBar
  (Widget|SetVisibility (UserInterface|GetUserWidgetObject (Variables|Default|GetHealthBar)) "Visible")
  (|CallParentFunction))

(event EventHideHealthBar
  (Widget|SetVisibility (UserInterface|GetUserWidgetObject (Variables|Default|GetHealthBar)) "Hidden")
  (|CallParentFunction))

(fn ConstructionScript)