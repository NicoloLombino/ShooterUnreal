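; Mutant boss enemy that faces its target, picks weighted random melee or ranged attacks by range, and shows boss health bars.
; A Tick state machine handles timed AI chases and sine-arc jumps, while delayed montage attacks re-trigger attack selection.
; Arm and jump capsules deal melee damage through toggleable overlaps.
; Ranged attacks spawn explosions on the target or fireballs, always the triple volley at half health or below.
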(event OnComponentBeginOverlap(CapsuleR)
  (params (OverlappedComponent :type Primitive%20Component%20Object%20Reference) (OtherActor :type Actor%20Object%20Reference) (OtherComp :type Primitive%20Component%20Object%20Reference) (OtherBodyIndex :type Integer) (bFromSweep :type Boolean) (SweepResult :type Hit%20Result%20Structure%20%28by%20ref%29))
  (Class|EnemyMonster|AttackCollisionHit OtherActor (Variables|Default|GetRightArmDamage)))

(event OnComponentEndOverlap(CapsuleR)
  (params (OverlappedComponent :type Primitive%20Component%20Object%20Reference) (OtherActor :type Actor%20Object%20Reference) (OtherComp :type Primitive%20Component%20Object%20Reference) (OtherBodyIndex :type Integer))
  (CallFunction|DisableCollisionAfterDamage (Variables|Default|GetCapsule%20R) OtherActor))

(event OnComponentBeginOverlap(CapsuleL)
  (params (OverlappedComponent :type Primitive%20Component%20Object%20Reference) (OtherActor :type Actor%20Object%20Reference) (OtherComp :type Primitive%20Component%20Object%20Reference) (OtherBodyIndex :type Integer) (bFromSweep :type Boolean) (SweepResult :type Hit%20Result%20Structure%20%28by%20ref%29))
  (Class|EnemyMonster|AttackCollisionHit OtherActor (Variables|Default|GetLeftArmDamage)))

(event OnComponentEndOverlap(CapsuleL)
  (params (OverlappedComponent :type Primitive%20Component%20Object%20Reference) (OtherActor :type Actor%20Object%20Reference) (OtherComp :type Primitive%20Component%20Object%20Reference) (OtherBodyIndex :type Integer))
  (CallFunction|DisableCollisionAfterDamage (Variables|Default|GetCapsule%20L) OtherActor))

(event OnComponentBeginOverlap(CapsuleJump)
  (params (OverlappedComponent :type Primitive%20Component%20Object%20Reference) (OtherActor :type Actor%20Object%20Reference) (OtherComp :type Primitive%20Component%20Object%20Reference) (OtherBodyIndex :type Integer) (bFromSweep :type Boolean) (SweepResult :type Hit%20Result%20Structure%20%28by%20ref%29))
  (Class|EnemyMonster|AttackCollisionHit OtherActor 3e+01))

(event OnComponentEndOverlap(CapsuleJump)
  (params (OverlappedComponent :type Primitive%20Component%20Object%20Reference) (OtherActor :type Actor%20Object%20Reference) (OtherComp :type Primitive%20Component%20Object%20Reference) (OtherBodyIndex :type Integer))
  (CallFunction|DisableCollisionAfterDamage (Variables|Default|GetCapsule%20Jump) OtherActor))

(event OnComponentBeginOverlap(detectSphere)
  (params (OverlappedComponent :type Primitive%20Component%20Object%20Reference) (OtherActor :type Actor%20Object%20Reference) (OtherComp :type Primitive%20Component%20Object%20Reference) (OtherBodyIndex :type Integer) (bFromSweep :type Boolean) (SweepResult :type Hit%20Result%20Structure%20%28by%20ref%29))
  (if (== OtherActor (Game|Player|GetPlayerPawn 0))
    (CallFunction|ShowBossHealthBar)))

(event Custom|SetAttackCollider
  (params (Generate%20Overlap%20Events :type Boolean) (CapsuleCollision :type Capsule%20Component%20Object%20Reference))
  (Variables|/Script/Engine.PrimitiveComponent|SetbGenerateOverlapEvents CapsuleCollision Generate%20Overlap%20Events))

(event Custom|LookAtTarget
  (bind _target (Variables|Default|GetTarget))
  (bind _capsulecomponent (Variables|Default|GetCapsuleComponent))
  (if (Utilities|IsValid _target)
    (Transformation|SetWorldRotation _capsulecomponent (Math|Rotator|MakeRotator 0.0 0.0 (+ (.yaw (Math|Rotator|FindLookatRotation (Transformation|GetWorldLocation _capsulecomponent) (Transformation|GetActorLocation _target))) -9e+01)) false false)))

(event Custom|SetAttackColliderRight
  (params (Generate%20Overlap%20Events :type Boolean))
  (CallFunction|SetAttackCollider Generate%20Overlap%20Events (Variables|Default|GetCapsule%20R)))

(event Custom|ShowBossHealthBar
  (if (not (Variables|Default|GetHealthBarIsShow))
    (bind _returnvalue (UserInterface|CreateWidget "/Game/CoseMie/UI/WBP_MutantBossHealthBar.WBP_MutantBossHealthBar_C" (Game|GetPlayerController 0)))
    (UserInterface|Viewport|AddtoViewport _returnvalue 0)
    (Variables|/Game/CoseMie/UI/WBP_MutantBossHealthBar.WBP_MutantBossHealthBar_C|SetEnemyBoss _returnvalue self)
    (Variables|/Game/CoseMie/UI/WBP_MutantBossHealthBar.WBP_MutantBossHealthBar_C|SetKeyToSpawn _returnvalue (Variables|Default|GetKeyToSpawn))))

(event Custom|SetAttackColliderJump
  (params (Generate%20Overlap%20Events :type Boolean))
  (CallFunction|SetAttackCollider Generate%20Overlap%20Events (Variables|Default|GetCapsule%20Jump)))

(event Custom|ShotAllFireball
  (for _array_element (Utilities|Array|MakeArray (Variables|Default|GetFireShotScene) (Variables|Default|GetFireShotScene1) (Variables|Default|GetFireShotScene2))
    (Game|SpawnActorfromClass "/Game/CoseMie/Blueprint/BP_MutantBossRangeAttackFireBall.BP_MutantBossRangeAttackFireBall_C" (Transformation|GetWorldTransform _array_element) "Undefined" 0 0)))

(event Custom|ShotFireballSingle
  (bind _returnvalue (Game|SpawnActorfromClass "/Game/CoseMie/Blueprint/BP_MutantBossRangeAttackFireBall.BP_MutantBossRangeAttackFireBall_C" (Transformation|GetWorldTransform (Variables|Default|GetFireShotScene)) "Undefined" 0 0))
  (Variables|/Game/CoseMie/Blueprint/BP_MutantBossRangeAttackFireBall.BP_MutantBossRangeAttackFireBall_C|SetSpeed _returnvalue 8e+02))

(event Custom|HandleDeath
  (Variables|/Script/Engine.PrimitiveComponent|SetbGenerateOverlapEvents (Variables|Default|GetCapsule%20Jump) false)
  (Variables|/Script/Engine.PrimitiveComponent|SetbGenerateOverlapEvents (Variables|Default|GetCapsule%20R) false)
  (Variables|/Script/Engine.PrimitiveComponent|SetbGenerateOverlapEvents (Variables|Default|GetCapsule%20L) false))

(event Custom|CheckDistanceFromPlayerAndDoAttack
  (Variables|Default|SetCanAttack false)
  (if (Variables|Default|GetisInAttackRange)
    (if (> (Math|Random|RandomIntegerinRange 0 5) 0)
      (CallFunction|DoRandomMeleeAttack :!label _label)
      (else
        (CallFunction|RandomRangeAttack :!label _label_2)))
    (Class|EnemyMonster|EnableMovement)
    (Variables|Default|SetHasRunToPlayer false)
    (elif (Utilities|IsValid (Variables|Default|GetTarget))
      (switch int (Math|Random|RandomIntegerinRange 0 2)
        (:Default
          (goto _label_2))
        (:0
          (goto _label_2))
        (:1
          (goto _label_2))
        (:2
          (if (Variables|Default|GetHasRunToPlayer)
            (switch int (Math|Random|RandomIntegerinRange 0 1)
              (:0
                (goto _label))
              (:1
                (CallFunction|CheckDistancefromPlayerandDoAttack)))
            (else
              (Variables|Default|SetHasRunToPlayer true)
              (Development|PrintString "FOLLOW START")
              (Class|EnemyMonster|EnableMovement)
              (Variables|Default|SetMaxRunTime (Math|Random|RandomFloatinRange 3.0 5.0))
              (CallFunction|ResetRuntoPlayer)
              (Variables|Default|SetMutantState "NewEnumerator3")
              (Animation|StopAnimMontage "/Game/CoseMie/Actors/MutantBoss/AM_MutantRangeAttacks.AM_MutantRangeAttacks"))))))))

(event Custom|DisableCollisionAfterDamage
  (params (CapsuleCollision :type Capsule%20Component%20Object%20Reference) (OtherObject :type Object%20Object%20Reference))
  (Utilities|Casting|CastToBP_PlayerBaseDoozy OtherObject)
  (if (Variables|Default|GetDoingSingleAttack)
    (CallFunction|SetAttackCollider false CapsuleCollision)))

(event Custom|HandleRangeAttack1
  ;[1 1 1] ATTACKS RANGE HANDLE
  (Game|SpawnActorfromClass "/Game/CoseMie/Blueprint/BP_MutantBossRangeAttackExplosion.BP_MutantBossRangeAttackExplosion_C" (Math|Conversions|ToTransform(Vector) (Transformation|GetActorLocation (Variables|Default|GetTarget))) "Undefined" 0 0))

(event Custom|HandleRangeAttack2
  ;[1 1 1] ATTACKS RANGE HANDLE
  (if (<= (Variables|Default|GetcurrentHealth) (/ (Variables|Default|GetmaxHealth) 2.0))
    (CallFunction|ShotAllFireball :!label _label)
    (elif (> (Math|Random|RandomIntegerinRange 0 2) 0)
      (CallFunction|ShotFireballSingle)
      (else
        (goto _label)))))

(event Custom|DoRandomMeleeAttack
  (bind _attacktimertogive (|CheckRageAndSetAttackTimer))
  (bind _attackcombodamage (Variables|Default|GetAttackComboDamage))
  (switch int (Math|Random|RandomIntegerinRange 0 5)
    (:Default
      (Animation|PlayAnimMontage "/Game/CoseMie/Actors/MutantBoss/AM_MutantAttacks.AM_MutantAttacks" 1.0 "AttackBase" :!label _label)
      (Audio|PlaySound2D "/Game/CoseMie/Sounds/Enemies/Boss/BossAttackBase.BossAttackBase" 1.0 1.0 0.0 0 0)
      (Variables|Default|SetDoingSingleAttack true)
      (Variables|Default|SetMutantState "NewEnumerator1")
      (Variables|Default|SetLeftArmDamage (Variables|Default|GetAttackBaseDamage))
      (Utilities|FlowControl|Delay (+ 2.5 _attacktimertogive))
      (Variables|Default|SetCanAttack true)
      (Variables|Default|SetDoingSingleAttack false))
    (:0
      (goto _label))
    (:1
      (goto _label))
    (:2
      (goto _label))
    (:3
      (Animation|PlayAnimMontage "/Game/CoseMie/Actors/MutantBoss/AM_MutantAttacks.AM_MutantAttacks" 1.0 "Attack360" :!label _label_2)
      (Audio|PlaySound2D "/Game/CoseMie/Sounds/Enemies/Boss/BossAttackBase.BossAttackBase" 1.0 1.0 0.0 0 0)
      (Variables|Default|SetDoingSingleAttack true)
      (Variables|Default|SetMutantState "NewEnumerator1")
      (Variables|Default|SetLeftArmDamage (Variables|Default|GetAttack360Damage))
      (Utilities|FlowControl|Delay (+ 2.5 _attacktimertogive))
      (Variables|Default|SetCanAttack true)
      (Variables|Default|SetDoingSingleAttack false))
    (:4
      (goto _label_2))
    (:5
      (Animation|PlayAnimMontage "/Game/CoseMie/Actors/MutantBoss/AM_MutantAttacks.AM_MutantAttacks" 1.0 "AttackCombo")
      (Audio|PlaySound2D "/Game/CoseMie/Sounds/Enemies/Boss/Boss_Combo.Boss_Combo" 1.0 1.0 0.0 0 0)
      (Variables|Default|SetMutantState "NewEnumerator1")
      (Variables|Default|SetLeftArmDamage _attackcombodamage)
      (Variables|Default|SetRightArmDamage (/ _attackcombodamage 2.0))
      (Utilities|FlowControl|Delay (+ 2.5 _attacktimertogive))
      (Variables|Default|SetCanAttack true)))
  (CallFunction|CheckDistancefromPlayerandDoAttack))

(event Custom|ResetRunToPlayer
  (Utilities|FlowControl|DoOnce false) ; enters at Reset
)

(event Custom|RandomRangeAttack
  (bind _attacktimertogive (|CheckRageAndSetAttackTimer_2))
  (switch int (Math|Random|RandomIntegerinRange 0 6)
    (:Default
      (Animation|PlayAnimMontage "/Game/CoseMie/Actors/MutantBoss/AM_MutantRangeAttacks.AM_MutantRangeAttacks" 1.5 "JumpAttack" :!label _label)
      (Audio|PlaySound2D "/Game/CoseMie/Sounds/Enemies/Boss/442957__qubodup__monster-attack.442957__qubodup__monster-attack" 5.0 1.0 0.0 0 0)
      (Variables|Default|SetDoingSingleAttack true)
      (Variables|Default|SetJumpEndLocation (Transformation|GetActorLocation (Variables|Default|GetTarget)))
      (Variables|Default|SetJumpStartLocation (Transformation|GetActorLocation))
      (Variables|Default|SetIsJumpingAttack true)
      (Variables|Default|SetMutantState "NewEnumerator2")
      (Utilities|FlowControl|Delay (+ 4.5 _attacktimertogive))
      (Variables|Default|SetCanAttack true)
      (Variables|Default|SetIsJumpingAttack false)
      (Variables|Default|SetJumpTimer 0.0)
      (Variables|Default|SetDoingSingleAttack false))
    (:0
      (Animation|PlayAnimMontage "/Game/CoseMie/Actors/MutantBoss/AM_MutantRangeAttacks.AM_MutantRangeAttacks" 1.0 "AttackRange1" :!label _label_2)
      (Audio|PlaySound2D "/Game/CoseMie/Sounds/Enemies/Boss/464952__giddster__monster-roar-3.464952__giddster__monster-roar-3" 1.0 1.0 0.0 0 0)
      (Variables|Default|SetDoingSingleAttack true)
      (CallFunction|HandleRangeAttack1)
      (Variables|Default|SetMutantState "NewEnumerator1")
      (Variables|Default|SetRightArmDamage 5.0)
      (Utilities|FlowControl|Delay (+ 1.5 _attacktimertogive))
      (Variables|Default|SetCanAttack true)
      (Variables|Default|SetDoingSingleAttack false)
      (CallFunction|CheckDistancefromPlayerandDoAttack :!label _label_3))
    (:1
      (goto _label_2))
    (:2
      (goto _label_2))
    (:3
      (Animation|PlayAnimMontage "/Game/CoseMie/Actors/MutantBoss/AM_MutantRangeAttacks.AM_MutantRangeAttacks" 1.0 "AttackRange2" :!label _label_4)
      (Audio|PlaySound2D "/Game/CoseMie/Sounds/Enemies/Boss/Boss.Boss" 3.0 1.0 0.0 0 0)
      (Variables|Default|SetDoingSingleAttack true)
      (Variables|Default|SetMutantState "NewEnumerator1")
      (Variables|Default|SetRightArmDamage 5.0)
      (Variables|Default|SetLeftArmDamage 5.0)
      (Utilities|FlowControl|Delay (+ 4.5 _attacktimertogive))
      (Variables|Default|SetCanAttack true)
      (Variables|Default|SetDoingSingleAttack false)
      (goto _label_3))
    (:4
      (goto _label_4))
    (:5
      (goto _label))
    (:6
      (goto _label))))

(event Custom|SetAttackColliderLeft
  (params (Generate%20Overlap%20Events :type Boolean))
  (CallFunction|SetAttackCollider Generate%20Overlap%20Events (Variables|Default|GetCapsule%20L)))

(event EventBeginPlay
  (bind _asbp_enemy_widget_life (Utilities|Casting|CastToBP_EnemyWidgetLife (UserInterface|GetUserWidgetObject (Variables|Default|GetHealthBar))))
  (Variables|/Game/CoseMie/UI/BP_EnemyWidgetLife.BP_EnemyWidgetLife_C|SetEnemy _asbp_enemy_widget_life self)
  (Widget|SetVisibility (UserInterface|GetUserWidgetObject (Variables|Default|GetHealthBar)) "Hidden"))

(event EventTick
  (params (DeltaSeconds :type Float%20%28single-precision%29))
  (if (> (Variables|Default|GetcurrentHealth) 0.0)
    (CallFunction|LookatTarget)
    (if (Utilities|IsValid (Variables|Default|GetTarget))
      (switch Utilities|FlowControl|Switch|SwitchonENUM_MutantBossState (Variables|Default|GetMutantState)
        (:NewEnumerator0
          (Utilities|FlowControl|DoOnce false
            (:Completed
              (CallFunction|CheckDistancefromPlayerandDoAttack))))
        (:NewEnumerator2
          (if (< (Variables|Default|GetJumpTimer) 1.0)
            (Variables|Default|SetJumpTimer (+ (Variables|Default|GetJumpTimer) DeltaSeconds))
            (Transformation|SetActorLocation (Math|Vector|MakeVector (.x (Math|Vector|Lerp(Vector) (Variables|Default|GetJumpStartLocation) (Variables|Default|GetJumpEndLocation) (Math|Float|Clamp(Float) (/ (Variables|Default|GetJumpTimer) 1.0)))) (.y (Math|Vector|Lerp(Vector) (Variables|Default|GetJumpStartLocation) (Variables|Default|GetJumpEndLocation) (Math|Float|Clamp(Float) (/ (Variables|Default|GetJumpTimer) 1.0)))) (+ (.z (Math|Vector|Lerp(Vector) (Variables|Default|GetJumpStartLocation) (Variables|Default|GetJumpEndLocation) (Math|Float|Clamp(Float) (/ (Variables|Default|GetJumpTimer) 1.0)))) (* 3e+02 (Math|Trig|Sin(Radians) (* (/ (Variables|Default|GetJumpTimer) 1.0) (Math|Trig|GetPI)))))) false false)
            (else
              (Variables|Default|SetMutantState "NewEnumerator0")
              (CallFunction|CheckDistancefromPlayerandDoAttack))))
        (:NewEnumerator3
          (Variables|Default|SetRunTimer (+ (Variables|Default|GetRunTimer) DeltaSeconds))
          (Class|EnemyMonster|EnableMovement)
          (if (< (Variables|Default|GetRunTimer) (Variables|Default|GetMaxRunTime))
            (Utilities|FlowControl|DoOnce false
              (:Completed
                (AI|AIMoveTo self (Transformation|GetActorLocation (Variables|Default|GetTarget)) 0 5.0 true
                  (:OnSuccess
                    (Development|PrintString "SUCCESS")
                    (Variables|Default|SetRunTimer 3e+01)
                    (CallFunction|CheckDistancefromPlayerandDoAttack))
                  (:OnFail
                    (Development|PrintString "FAIL")
                    (CallFunction|ResetRuntoPlayer)))))
            (else
              (Variables|Default|SetRunTimer 0.0)
              (CallFunction|CheckDistancefromPlayerandDoAttack))))))
    (else
      (Utilities|FlowControl|DoOnce false
        (:Completed
          (CallFunction|HandleDeath))))))

(event EventShowHealthBar
  (Widget|SetVisibility (UserInterface|GetUserWidgetObject (Variables|Default|GetHealthBar)) "Visible")
  (|CallParentFunction)
  (CallFunction|ShowBossHealthBar))

(event EventHideHealthBar
  (Widget|SetVisibility (UserInterface|GetUserWidgetObject (Variables|Default|GetHealthBar)) "Hidden")
  (|CallParentFunction))

(fn ConstructionScript)