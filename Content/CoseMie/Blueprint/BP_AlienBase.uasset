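; BP_AlienBase is an alien enemy with a health bar widget and a melee attack.
; While alive and in range, Tick turns the capsule toward the target, plays the attack montage and sound, then waits montage length plus AttackTimer before attacking again.
; A toggleable sphere collider passes overlapped actors and Damage to AttackCollisionHit.
; The health bar binds to the enemy on BeginPlay, starts hidden, and shows or hides through events.
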(event OnComponentBeginOverlap(Sphere)
  (params (OverlappedComponent :type Primitive%20Component%20Object%20Reference) (OtherActor :type Actor%20Object%20Reference) (OtherComp :type Primitive%20Component%20Object%20Reference) (OtherBodyIndex :type Integer) (bFromSweep :type Boolean) (SweepResult :type Hit%20Result%20Structure%20%28by%20ref%29))
  (Class|EnemyMonster|AttackCollisionHit OtherActor (Variables|Default|Getdamage)))

(event Custom|SetAttackCollider
  (params (Generate%20Overlap%20Events :type Boolean))
  (Variables|/Script/Engine.PrimitiveComponent|SetbGenerateOverlapEvents (Variables|Default|GetSphere) Generate%20Overlap%20Events))

(event Custom|LookAtTarget
  (bind _target (Variables|Default|GetTarget))
  (bind _capsulecomponent (Variables|Default|GetCapsuleComponent))
  (if (Utilities|IsValid _target)
    (Transformation|SetWorldRotation _capsulecomponent (Math|Rotator|FindLookatRotation (Transformation|GetWorldLocation _capsulecomponent) (Transformation|GetActorLocation _target)) false false)))

(event EventBeginPlay
  (bind _asbp_enemy_widget_life (Utilities|Casting|CastToBP_EnemyWidgetLife (UserInterface|GetUserWidgetObject (Variables|Default|GetHealthBar))))
  (Variables|/Game/CoseMie/UI/BP_EnemyWidgetLife.BP_EnemyWidgetLife_C|SetEnemy _asbp_enemy_widget_life self)
  (Widget|SetVisibility (UserInterface|GetUserWidgetObject (Variables|Default|GetHealthBar)) "Hidden"))

(event Collision|EventActorBeginOverlap
  (params (OtherActor :type Actor%20Object%20Reference)))

(event EventTick
  (params (DeltaSeconds :type Float%20%28single-precision%29))
  (if (> (Variables|Default|GetcurrentHealth) 0.0)
    (if (Variables|Default|GetisInAttackRange)
      (if (Variables|Default|GetCanAttack)
        (Variables|Default|SetCanAttack false)
        (CallFunction|LookatTarget)
        (bind _returnvalue (Animation|PlayAnimMontage "/Game/CoseMie/Actors/AlienMixamo/AlienBaseAttack1Montage.AlienBaseAttack1Montage" 1.0 "None"))
        (Audio|PlaySound2D "/Game/CoseMie/Actors/AlienMixamo/Sound/alien_attack_1.alien_attack_1" 5.0 1.0 0.0 0 0)
        (Utilities|FlowControl|Delay (+ _returnvalue (Variables|Default|GetAttackTimer)))
        (Variables|Default|SetCanAttack true)))))

(event EventShowHealthBar
  (Widget|SetVisibility (UserInterface|GetUserWidgetObject (Variables|Default|GetHealthBar)) "Visible")
  (|CallParentFunction))

(event EventHideHealthBar
  (Widget|SetVisibility (UserInterface|GetUserWidgetObject (Variables|Default|GetHealthBar)) "Hidden")
  (|CallParentFunction))

(fn ConstructionScript)