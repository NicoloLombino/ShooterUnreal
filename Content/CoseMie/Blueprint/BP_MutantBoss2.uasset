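; Mutant boss enemy that attacks a target in range with either a melee strike or a damage-over-time vomit area.
; Tick faces the target and randomly plays the Attack or less frequent Vomit montage section, then waits out a cooldown.
; A toggled sphere deals melee hits, while a timeline grows the vomit particles and cone, whose overlaps start and stop player damage.
; It also links and toggles its widget health bar.
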(event OnComponentBeginOverlap(Cone)
  (params (OverlappedComponent :type Primitive%20Component%20Object%20Reference) (OtherActor :type Actor%20Object%20Reference) (OtherComp :type Primitive%20Component%20Object%20Reference) (OtherBodyIndex :type Integer) (bFromSweep :type Boolean) (SweepResult :type Hit%20Result%20Structure%20%28by%20ref%29))
  (bind _asbp_player_base_doozy (Utilities|Casting|CastToBP_PlayerBaseDoozy OtherActor))
  (Class|PlayerBase|HandleEnteronVomitArea _asbp_player_base_doozy (Variables|Default|GetVomitDamage) (Variables|Default|GetVomitDamageRateTime)))

(event OnComponentBeginOverlap(Sphere)
  (params (OverlappedComponent :type Primitive%20Component%20Object%20Reference) (OtherActor :type Actor%20Object%20Reference) (OtherComp :type Primitive%20Component%20Object%20Reference) (OtherBodyIndex :type Integer) (bFromSweep :type Boolean) (SweepResult :type Hit%20Result%20Structure%20%28by%20ref%29))
  (Class|EnemyMonster|AttackCollisionHit OtherActor (Variables|Default|Getdamage)))

(event OnComponentEndOverlap(Cone)
  (params (OverlappedComponent :type Primitive%20Component%20Object%20Reference) (OtherActor :type Actor%20Object%20Reference) (OtherComp :type Primitive%20Component%20Object%20Reference) (OtherBodyIndex :type Integer))
  (bind _asbp_player_base_doozy (Utilities|Casting|CastToBP_PlayerBaseDoozy OtherActor))
  (Class|PlayerBase|HandleExitfromVomitArea _asbp_player_base_doozy))

(event Custom|SetAttackCollider
  (params (Generate%20Overlap%20Events :type Boolean))
  (Variables|/Script/Engine.PrimitiveComponent|SetbGenerateOverlapEvents (Variables|Default|GetSphere) Generate%20Overlap%20Events))

(event Custom|LookAtTarget
  (bind _target (Variables|Default|GetTarget))
  (bind _capsulecomponent (Variables|Default|GetCapsuleComponent))
  (if (Utilities|IsValid _target)
    (Transformation|SetWorldRotation _capsulecomponent (Math|Rotator|FindLookatRotation (Transformation|GetWorldLocation _capsulecomponent) (Transformation|GetActorLocation _target)) false false)))

(event Custom|HandleVomitAttack
  (bind _cone (Variables|Default|GetCone))
  (Rendering|SetVisibility (Variables|Default|GetParticleSystem) true false)
  (Variables|/Script/Engine.PrimitiveComponent|SetbGenerateOverlapEvents (Variables|Default|GetCone) true)
  (bind _vomitsize (Timeline|Timeline_0 Play)
    (:Update
      (Transformation|SetWorldScale3D (Variables|Default|GetParticleSystem) (/ (Math|Vector|MakeVector (Math|Float|Lerp 0.0 2.0 _vomitsize) (Math|Float|Lerp 0.0 2.0 _vomitsize) (Math|Float|Lerp 0.0 2.0 _vomitsize)) "2.000000,2.000000,2.000000"))
      (Transformation|SetWorldScale3D _cone (Math|Vector|MakeVector (Math|Float|Lerp 0.0 2.0 _vomitsize) (Math|Float|Lerp 0.0 2.0 _vomitsize) (Math|Float|Lerp 0.0 2.0 _vomitsize)))
      (Transformation|SetRelativeLocation _cone (Math|Vector|MakeVector 0.0 0.0 (Math|Float|Lerp 4e+01 9e+01 _vomitsize)) false false))))

(event Custom|StopVomitAttack
  (Rendering|SetVisibility (Variables|Default|GetParticleSystem) false false)
  (Variables|/Script/Engine.PrimitiveComponent|SetbGenerateOverlapEvents (Variables|Default|GetCone) false))

(event EventBeginPlay
  (bind _asbp_enemy_widget_life (Utilities|Casting|CastToBP_EnemyWidgetLife (UserInterface|GetUserWidgetObject (Variables|Default|GetHealthBar))))
  (Variables|/Game/CoseMie/UI/BP_EnemyWidgetLife.BP_EnemyWidgetLife_C|SetEnemy _asbp_enemy_widget_life self)
  (Widget|SetVisibility (UserInterface|GetUserWidgetObject (Variables|Default|GetHealthBar)) "Hidden"))

(event Collision|EventActorBeginOverlap
  (params (OtherActor :type Actor%20Object%20Reference)))

(event EventTick
  (params (DeltaSeconds :type Float%20%28single-precision%29))
  (if (> (Variables|Default|GetcurrentHealth) 0.0)
    (if (Variables|Default|GetisInAttackRange)
      (if (Variables|Default|GetCanAttack)
        (Variables|Default|SetCanAttack false)
        (CallFunction|LookatTarget)
        (switch int (Math|Random|RandomIntegerinRange 0 2)
          (:Default
            (bind _returnvalue (Animation|PlayAnimMontage "/Game/CoseMie/Actors/ZombiLikeMixamo/AM_ZombiMutantAttack1.AM_ZombiMutantAttack1" 1.0 "Attack" :!label _label))
            (Utilities|FlowControl|Delay (+ _returnvalue (Variables|Default|GetAttackTimer)))
            (Variables|Default|SetCanAttack true))
          (:0
            (goto _label))
          (:1
            (goto _label))
          (:2
            (bind _returnvalue_2 (Animation|PlayAnimMontage "/Game/CoseMie/Actors/ZombiLikeMixamo/AM_ZombiMutantAttack1.AM_ZombiMutantAttack1" 1.0 "Vomit"))
            (Utilities|FlowControl|Delay (+ _returnvalue_2 (Variables|Default|GetVomitAttackTimer)))
            (Variables|Default|SetCanAttack true)))))))

(event EventShowHealthBar
  (Widget|SetVisibility (UserInterface|GetUserWidgetObject (Variables|Default|GetHealthBar)) "Visible")
  (|CallParentFunction))

(event EventHideHealthBar
  (Widget|SetVisibility (UserInterface|GetUserWidgetObject (Variables|Default|GetHealthBar)) "Hidden")
  (|CallParentFunction))

(fn ConstructionScript)