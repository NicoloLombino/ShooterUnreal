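; Interactable door actor that the player opens with the E key, provided its IsOpen flag is set.
; On BeginPlay, a signal sphere takes an unlock or lock material based on that flag.
; A box overlap enables input only while the player character is inside.
; Pressing E passes a DoOnce and plays a timeline that lerps Door1's yaw from start to end rotation, with no closing logic.
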(event OnComponentBeginOverlap(Box)
  (params (OverlappedComponent :type Primitive%20Component%20Object%20Reference) (OtherActor :type Actor%20Object%20Reference) (OtherComp :type Primitive%20Component%20Object%20Reference) (OtherBodyIndex :type Integer) (bFromSweep :type Boolean) (SweepResult :type Hit%20Result%20Structure%20%28by%20ref%29))
  (if (== OtherActor (Game|GetPlayerCharacter 0))
    (Input|EnableInput (Game|GetPlayerController 0))))

(event OnComponentEndOverlap(Box)
  (params (OverlappedComponent :type Primitive%20Component%20Object%20Reference) (OtherActor :type Actor%20Object%20Reference) (OtherComp :type Primitive%20Component%20Object%20Reference) (OtherBodyIndex :type Integer))
  (if (== OtherActor (Game|GetPlayerCharacter 0))
    (Input|DisableInput (Game|GetPlayerController 0))))

(event EventBeginPlay
  (bind _sphere (Variables|Default|GetSphere))
  (Variables|Default|SetSignalMesh (Variables|Default|GetSphere))
  (if (Variables|Default|GetisOpen)
    (Rendering|Material|SetMaterial _sphere 0 (Variables|Default|GetUnlockMaterial))
    (else
      (Rendering|Material|SetMaterial _sphere 0 (Variables|Default|GetLockMaterial)))))

(event Input|KeyboardEvents|E
  (params (Key :type Key%20Structure :default "None"))
  (:Pressed
    (if (Variables|Default|GetisOpen)
      (Utilities|FlowControl|DoOnce false
        (:Completed
          (bind _opendoor (Timeline|Timeline Play)
            (:Update
              (Transformation|SetRelativeRotation (Variables|Default|GetDoor1) (Math|Rotator|MakeRotator 0.0 0.0 (Math|Float|Lerp (Variables|Default|GetStartDoorRotation) (Variables|Default|GetEndDoorRotation) _opendoor)) false false))))))))

(fn ConstructionScript)